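; BP_CustomizableCharacter is a character creation Blueprint that holds body shape values and a spring-arm camera.
; On BeginPlay it calls ApplyBodyMorphs, which only prints the breast, butt and height values as formatted text, without changing any mesh.
; UpdateCameraTransform then sets the spring arm's rotation, length and vertical offset from the camera variables, overriding the arm length BeginPlay just set.
; Tick, overlap and construction script are empty.
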(event EventBeginPlay
  (CallFunction|ApplyBodyMorphs)
  (Variables|/Script/Engine.SpringArmComponent|SetTargetArmLength (Variables|Default|GetCameraSpringArm) 5e+02)
  (CallFunction|UpdateCameraTransform))

(event Collision|EventActorBeginOverlap
  (params (OtherActor :type Actor%20Object%20Reference)))

(event EventTick
  (params (DeltaSeconds :type Float%20%28single-precision%29)))

(fn ConstructionScript)

(fn ApplyBodyMorphs
  (Development|PrintString (Utilities|String|ToString(Text) (Utilities|Text|FormatText (Utilities|Text|ToText(Float) (Variables|Default|GetBreastSize) "HalfToEven") (Utilities|Text|ToText(Float) (Variables|Default|GetButtSize) "HalfToEven") (Variables|Default|GetHeight)))))

(fn UpdateCameraTransform
  (Transformation|SetRelativeRotation (Variables|Default|GetCameraSpringArm) (Math|Rotator|MakeRotator 0.0 (Variables|Default|GetCameraPitch) (Variables|Default|GetCameraYaw)) false false)
  (Variables|/Script/Engine.SpringArmComponent|SetTargetArmLength (Variables|Default|GetCameraSpringArm) (Variables|Default|GetCameraDistance))
  (Transformation|SetRelativeLocation (Variables|Default|GetCameraSpringArm) (Math|Vector|MakeVector 0.0 0.0 (Variables|Default|GetCameraHeight)) false false))