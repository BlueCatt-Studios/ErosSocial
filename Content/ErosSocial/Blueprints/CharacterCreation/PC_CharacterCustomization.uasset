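; Player controller for the character customization screen that finds the level's BP_CustomizableCharacter and makes it the view target.
; Right-drag orbits the camera, middle-drag adjusts its height, the wheel zooms, and left-dragging on the character (cursor trace) spins its body mesh.
; Mouse axes write clamped pitch, height and distance plus free yaw onto the character, whose UpdateCameraTransform applies them.
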(event EventBeginPlay
  (Development|PrintString "\"PC BeginPlay Started\"" true true "(R=0.969375,G=1.000000,B=0.000000,A=1.000000)")
  (bind _returnvalue (Actor|GetActorOfClass "/Game/ErosSocial/Blueprints/CharacterCreation/BP_CustomizableCharacter.BP_CustomizableCharacter_C"))
  (bind _output_get (Variables|Default|SetCustomizableCharacterRef _returnvalue))
  (Development|PrintString "\"Character Reference Set\"")
  (if (Utilities|IsValid _output_get)
    (Development|PrintString "Setting View Target to Character" true true "(R=0.092793,G=1.000000,B=0.156864,A=1.000000)")
    (Game|Player|SetViewTargetwithBlend (Variables|Default|GetCustomizableCharacterRef) 0.0 "VTBlend_Linear" 0.0 false)
    (else
      (Development|PrintString "ERROR: CustomizableCharacter not found in level!" true true "(R=1.000000,G=0.000000,B=0.446249,A=1.000000)"))))

(event EventTick
  (params (DeltaSeconds :type Float%20%28single-precision%29)))

(event Input|MouseEvents|MouseX
  (params (AxisValue :type Float%20%28single-precision%29))
  (if (Variables|/Game/ErosSocial/Blueprints/CharacterCreation/BP_CustomizableCharacter.BP_CustomizableCharacter_C|GetIsRotatingCharacter (Variables|Default|GetCustomizableCharacterRef))
    (Transformation|SetRelativeRotation (Variables|/Game/ErosSocial/Blueprints/CharacterCreation/BP_CustomizableCharacter.BP_CustomizableCharacter_C|GetBodyMesh (Variables|Default|GetCustomizableCharacterRef)) (Math|Rotator|MakeRotator 0.0 0.0 (+ (.Yaw (Math|Rotator|BreakRotator (Variables|/Script/Engine.SceneComponent|GetRelativeRotation (Variables|/Game/ErosSocial/Blueprints/CharacterCreation/BP_CustomizableCharacter.BP_CustomizableCharacter_C|GetBodyMesh (Variables|Default|GetCustomizableCharacterRef))))) (* AxisValue -5.0))) false false)
    (elif (Variables|Default|GetIsRotatingCamera)
      (Variables|/Game/ErosSocial/Blueprints/CharacterCreation/BP_CustomizableCharacter.BP_CustomizableCharacter_C|SetCameraYaw (Variables|Default|GetCustomizableCharacterRef) (+ (Variables|/Game/ErosSocial/Blueprints/CharacterCreation/BP_CustomizableCharacter.BP_CustomizableCharacter_C|GetCameraYaw (Variables|Default|GetCustomizableCharacterRef)) (* AxisValue -2.0)))
      (Default|UpdateCameraTransform (Variables|Default|GetCustomizableCharacterRef)))))

(event Input|MouseEvents|MouseWheelAxis
  (params (AxisValue :type Float%20%28single-precision%29))
  (Variables|/Game/ErosSocial/Blueprints/CharacterCreation/BP_CustomizableCharacter.BP_CustomizableCharacter_C|SetCameraDistance (Variables|Default|GetCustomizableCharacterRef) (Math|Float|Clamp(Float) (- (Variables|/Game/ErosSocial/Blueprints/CharacterCreation/BP_CustomizableCharacter.BP_CustomizableCharacter_C|GetCameraDistance (Variables|Default|GetCustomizableCharacterRef)) (* AxisValue 5e+01)) 2e+02 8e+02))
  (Default|UpdateCameraTransform (Variables|Default|GetCustomizableCharacterRef)))

(event Input|MouseEvents|MouseY
  (params (AxisValue :type Float%20%28single-precision%29))
  (if (Variables|/Game/ErosSocial/Blueprints/CharacterCreation/BP_CustomizableCharacter.BP_CustomizableCharacter_C|GetIsAdjustingHeight (Variables|Default|GetCustomizableCharacterRef))
    (Variables|/Game/ErosSocial/Blueprints/CharacterCreation/BP_CustomizableCharacter.BP_CustomizableCharacter_C|SetCameraHeight (Variables|Default|GetCustomizableCharacterRef) (Math|Float|Clamp(Float) (+ (* AxisValue 5.0) (Variables|/Game/ErosSocial/Blueprints/CharacterCreation/BP_CustomizableCharacter.BP_CustomizableCharacter_C|GetCameraHeight (Variables|Default|GetCustomizableCharacterRef))) 1e+02 2.5e+02))
    (Default|UpdateCameraTransform (Variables|Default|GetCustomizableCharacterRef))
    (elif (Variables|Default|GetIsRotatingCamera)
      (Variables|/Game/ErosSocial/Blueprints/CharacterCreation/BP_CustomizableCharacter.BP_CustomizableCharacter_C|SetCameraPitch (Variables|Default|GetCustomizableCharacterRef) (Math|Float|Clamp(Float) (+ (Variables|/Game/ErosSocial/Blueprints/CharacterCreation/BP_CustomizableCharacter.BP_CustomizableCharacter_C|GetCameraPitch (Variables|Default|GetCustomizableCharacterRef)) (* AxisValue -2.0)) -8e+01 0.0))
      (Default|UpdateCameraTransform (Variables|Default|GetCustomizableCharacterRef)))))

(event Input|MouseEvents|RightMouseButton
  (params (Key :type Key%20Structure :default "None"))
  (:Pressed
    (Variables|Default|SetIsRotatingCamera true))
  (:Released
    (Variables|Default|SetIsRotatingCamera false)))

(event Input|MouseEvents|MiddleMouseButton
  (params (Key :type Key%20Structure :default "None"))
  (:Pressed
    (Variables|/Game/ErosSocial/Blueprints/CharacterCreation/BP_CustomizableCharacter.BP_CustomizableCharacter_C|SetIsAdjustingHeight (Variables|Default|GetCustomizableCharacterRef) true)
    (Variables|Default|SetbShowMouseCursor false))
  (:Released
    (Variables|/Game/ErosSocial/Blueprints/CharacterCreation/BP_CustomizableCharacter.BP_CustomizableCharacter_C|SetIsAdjustingHeight (Variables|Default|GetCustomizableCharacterRef) false)
    (Variables|Default|SetbShowMouseCursor true)))

(event Input|MouseEvents|LeftMouseButton
  (params (Key :type Key%20Structure :default "None"))
  (:Pressed
    (if (== (.HitActor (Collision|BreakHitResult (.HitResult (Game|Player|GetHitResultUnderCursorbyChannel "TraceTypeQuery1" true)))) (Variables|Default|GetCustomizableCharacterRef))
      (Development|PrintString "\"CLICOU NO CHARACTER! \"")
      (Variables|/Game/ErosSocial/Blueprints/CharacterCreation/BP_CustomizableCharacter.BP_CustomizableCharacter_C|SetIsRotatingCharacter (Variables|Default|GetCustomizableCharacterRef) true)
      (Variables|Default|SetbShowMouseCursor false)))
  (:Released
    (Variables|/Game/ErosSocial/Blueprints/CharacterCreation/BP_CustomizableCharacter.BP_CustomizableCharacter_C|SetIsRotatingCharacter (Variables|Default|GetCustomizableCharacterRef) false)
    (Variables|Default|SetbShowMouseCursor true)))

(fn ConstructionScript)